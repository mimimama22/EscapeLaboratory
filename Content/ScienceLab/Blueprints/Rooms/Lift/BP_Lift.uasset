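; Lift actor that carries its cabin vertically to a target floor height when its Box component is interacted with.
; Tick moves the root's Z toward PositionNextFloor at constant speed, then stops and opens both its own doors and those of the referenced LiftFloor.
; A MoveDoor timeline swings the two cabin doors in opposite yaw directions, playing to open and reversing to close.
; The target height is not set within this graph.
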(event `OpenDoors`
  (bind (_direction _newtrack_0) (`Timeline|MoveDoor` :!label _label)
    (:`Update`
      (bind _returnvalue (* _newtrack_0 20.0))
      (`SceneComponent.K2_SetRelativeRotation` (`self.SM_Lift02Door02`) (`KismetMathLibrary.MakeRotator` 0.0 0.0 _returnvalue) false false)
      (`SceneComponent.K2_SetRelativeRotation` (`self.SM_Lift02Door01`) (`KismetMathLibrary.MakeRotator` 0.0 0.0 (* _returnvalue -1.0)) false false))))

(event `CloseDoors`
  (goto _label :!via `Reverse`))

(event `/Game/BPI_Interaction.Interaction`
  (params (staticComponent :type "BoxComponent Object Reference"))
  (if (== staticComponent (`self.Box`))
    (set `self.MoveFloor` true)))

(event `self.ReceiveTick`
  (params (DeltaSeconds :type "Float (single-precision)"))
  (bind (_returnvalue_x _returnvalue_y _returnvalue_z) (`KismetMathLibrary.BreakVector` (`SceneComponent.K2_GetComponentLocation` (`self.DefaultSceneRoot`))))
  (bind _returnvalue (`KismetMathLibrary.FInterpTo_Constant` _returnvalue_z (`self.PositionNextFloor`) (`GameplayStatics.GetWorldDeltaSeconds`) 500.0))
  (if (`self.MoveFloor`)
    (`SceneComponent.K2_SetWorldLocation` (`self.DefaultSceneRoot`) (`KismetMathLibrary.MakeVector` _returnvalue_x _returnvalue_y _returnvalue) false false)
    (if (== _returnvalue (`self.PositionNextFloor`))
      (set `self.MoveFloor` false)
      (`self.OpenDoors`)
      (`/Game/ScienceLab/Blueprints/Rooms/Lift/BP_Lift04.opendoors` (`self.LiftFloorRef`)))))

(fn `UserConstructionScript`)